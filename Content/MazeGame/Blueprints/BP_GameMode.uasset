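; BP_GameMode is the maze game's game mode, tracking play time and handling the end of a run.
; While the game is running, Tick adds delta time to TotalTime on BP_GameInstance.
; EndGame fires only once per run, clearing the running flag, showing the WBP_FinalScore widget and disabling the first player controller's input.
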(event `self.ReceiveBeginPlay`)

(event `self.ReceiveTick`
  (params (DeltaSeconds :type "Float (single-precision)"))
  (if (`self.bGameIsRunning`)
    (bind _asbp_game_instance (cast `/Game/MazeGame/Blueprints/BP_GameInstance` (`GameplayStatics.GetGameInstance`)))
    (set `/Game/MazeGame/Blueprints/BP_GameInstance.TotalTime` (+ (`/Game/MazeGame/Blueprints/BP_GameInstance.TotalTime` _asbp_game_instance) DeltaSeconds) _asbp_game_instance)))

(event `EndGame`
  (if (`self.bGameIsRunning`)
    (set `self.bGameIsRunning` false)
    (bind _returnvalue (`|CreateWidget` "/Game/MazeGame/Blueprints/WBP_FinalScore.WBP_FinalScore_C"))
    (`UserWidget.AddToViewport` _returnvalue 0)
    (`self.DisableInput` (`GameplayStatics.GetPlayerController` 0) null)))

(fn `UserConstructionScript`)