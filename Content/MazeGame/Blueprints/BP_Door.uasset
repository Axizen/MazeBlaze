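; BP_Door is a maze game door whose color and mask are configured from a data table row.
; Its construction script creates a dynamic instance of M_BasicColor and applies it to the mesh.
; It then looks up the DoorDataHandle row, stores the row's Mask and sets the material's Color parameter.
; The event graph holds only disabled placeholder events, so all logic runs at construction.
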(fn `UserConstructionScript`
  (bind (_datatable _rowname) (break `DataTableRowHandle` (`self.DoorDataHandle`)))
  (bind _returnvalue (`KismetMaterialLibrary.CreateDynamicMaterialInstance` "/Game/MazeGame/Materials/M_BasicColor.M_BasicColor"))
  (bind _output_get (set `self.Material` _returnvalue))
  (`PrimitiveComponent.SetMaterial` (`self.Mesh`) 0 _output_get)
  (bind _returnvalue_2 (`|GetDataTableRow` _datatable _rowname)
    (:`then`
      (bind (_mask _color) (break `/Game/MazeGame/Data/FDoorDataRow` _returnvalue_2))
      (set `self.Mask` _mask)
      (`MaterialInstanceDynamic.SetVectorParameterValue` (`self.Material`) "Color" _color))))