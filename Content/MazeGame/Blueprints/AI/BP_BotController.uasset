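; BP_BotController is the controller for BP_Bot in MazeGame, linking the bot's key pickups to an on-screen HUD.
; On BeginPlay it creates a WBP_HUD widget and adds it to the viewport.
; It binds to the bot's OnPickupKey event on possess and unbinds on unpossess.
; Each pickup passes the key's name to the HUD to update its display.
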(event `self.ReceiveBeginPlay`
  (bind _returnvalue (`|CreateWidget` "/Game/MazeGame/Blueprints/WBP_HUD.WBP_HUD_C"))
  (bind _output_get (set `self.HUD` _returnvalue))
  (`UserWidget.AddToViewport` _output_get 0))

(event `self.ReceivePossess`
  (params (PossessedPawn :type "Pawn Object Reference"))
  (bind _asbp_bot (cast `/Game/MazeGame/Blueprints/AI/BP_Bot` PossessedPawn))
  (add `MazeGameCharacter.OnPickupKey` _asbp_bot (delegate `OnPickupKey`)))

(event `self.ReceiveUnPossess`
  (params (UnpossessedPawn :type "Pawn Object Reference"))
  (bind _asbp_bot (cast `/Game/MazeGame/Blueprints/AI/BP_Bot` UnpossessedPawn))
  (remove `MazeGameCharacter.OnPickupKey` _asbp_bot (delegate `OnPickupKey`)))

(event `OnPickupKey`
  (params (Key :type "MazeGameKey Object Reference"))
  (`/Game/MazeGame/Blueprints/WBP_HUD.UpdateKeyName` (`self.HUD`) (`MazeGameKey.GetKeyName` Key)))

(fn `UserConstructionScript`)