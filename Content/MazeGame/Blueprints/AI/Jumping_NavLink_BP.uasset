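; Smart nav link that makes AI bots jump to the link's destination in the maze game.
; When a BP_Bot reaches the link, it is launched with a velocity that overrides its current movement on all axes.
; CalculateVelocity solves the ballistic arc for a set JumpDuration, using linear horizontal speed and a vertical term that compensates for a hardcoded gravity constant.
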(event `self.ReceiveSmartLinkReached`
  (params (Agent :type "Actor Object Reference") (Destination :type "Vector Structure (by ref)"))
  (bind _asbp_bot (cast `/Game/MazeGame/Blueprints/AI/BP_Bot` Agent))
  (`/Engine/EditorBlueprintResources/StandardMacros.IsValid` _asbp_bot
    (:`Is Valid`
      (bind _velocity (`self.CalculateVelocity` Destination (`self.K2_GetActorLocation` _asbp_bot) (`self.JumpDuration`)))
      (`Character.LaunchCharacter` _asbp_bot _velocity true true))))

(fn `CalculateVelocity`
  (params (`Destination Location` :type "Vector Structure") (StartingLocation :type "Vector Structure") (Duration :type "Float (double-precision)"))
  (returns (Velocity :type "Vector Structure"))
  (locals (LocalDuration :type "Float (double-precision)"))
  (bind _localduration (`local.LocalDuration`))
  (set `local.LocalDuration` Duration)
  (return (`KismetMathLibrary.MakeVector` (/ (- (.x `Destination Location`) (.x StartingLocation)) _localduration) (/ (- (.y `Destination Location`) (.y StartingLocation)) _localduration) (/ (- (.z `Destination Location`) (+ (.z StartingLocation) (* (`KismetMathLibrary.Square` (`local.LocalDuration`)) -0.5 982.0))) (`local.LocalDuration`)))))

(fn `UserConstructionScript`)