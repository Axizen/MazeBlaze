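; Player controller for the maze game that owns the HUD and shows picked-up keys on it.
; On BeginPlay it creates WBP_HUD and adds it to the viewport.
; It binds to the possessed BP_MazeBlazeCharacter's OnPickupKey event and unbinds on unpossess.
; When a key is picked up, it passes the key's name to the HUD.
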(event `self.ReceiveBeginPlay`
  (bind _returnvalue (`|CreateWidget` "/Game/MazeGame/Blueprints/WBP_HUD.WBP_HUD_C" self))
  (bind _output_get (set `self.HUD` _returnvalue))
  (`UserWidget.AddToViewport` _output_get 0))

(event `self.ReceivePossess`
  (params (PossessedPawn :type "Pawn Object Reference"))
  (bind _asbp_maze_blaze_character (cast `/Game/MazeGame/Blueprints/BP_MazeBlazeCharacter` PossessedPawn))
  (add `MazeBlazeCharacter.OnPickupKey` _asbp_maze_blaze_character (delegate `OnPickupKey`)))

(event `self.ReceiveUnPossess`
  (params (UnpossessedPawn :type "Pawn Object Reference"))
  (bind _asbp_maze_blaze_character (cast `/Game/MazeGame/Blueprints/BP_MazeBlazeCharacter` UnpossessedPawn))
  (remove `MazeBlazeCharacter.OnPickupKey` _asbp_maze_blaze_character (delegate `OnPickupKey`)))

(event `OnPickupKey`
  (params (Key :type "MazeBlazeKey Object Reference"))
  (`/Game/MazeGame/Blueprints/WBP_HUD.UpdateKeyName` (`self.HUD`) (`MazeBlazeKey.GetKeyName` Key)))

(fn `UserConstructionScript`)