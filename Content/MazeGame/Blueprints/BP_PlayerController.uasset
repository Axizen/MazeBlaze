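; Player controller for the maze game that owns the HUD and reflects key pickups on screen.
; On BeginPlay it creates the WBP_HUD widget and adds it to the viewport.
; When it possesses or unpossesses a BP_Character, it binds or unbinds that character's OnPickupKey event.
; Each pickup passes the key's name to the HUD to update its key display.
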(event `self.ReceiveBeginPlay`
  (bind _returnvalue (`|CreateWidget` "/Game/MazeGame/Blueprints/WBP_HUD.WBP_HUD_C" self))
  (bind _output_get (set `self.HUD` _returnvalue))
  (`UserWidget.AddToViewport` _output_get 0))

(event `self.ReceivePossess`
  (params (PossessedPawn :type "Pawn Object Reference"))
  (bind _asbp_character (cast `/Game/MazeGame/Blueprints/BP_Character` PossessedPawn))
  (add `MazeGameCharacter.OnPickupKey` _asbp_character (delegate `OnPickupKey`)))

(event `self.ReceiveUnPossess`
  (params (UnpossessedPawn :type "Pawn Object Reference"))
  (bind _asbp_character (cast `/Game/MazeGame/Blueprints/BP_Character` UnpossessedPawn))
  (remove `MazeGameCharacter.OnPickupKey` _asbp_character (delegate `OnPickupKey`)))

(event `OnPickupKey`
  (params (Key :type "MazeGameKey Object Reference"))
  (`/Game/MazeGame/Blueprints/WBP_HUD.UpdateKeyName` (`self.HUD`) (`MazeGameKey.GetKeyName` Key)))

(fn `UserConstructionScript`)