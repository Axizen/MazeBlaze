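; BP_Key is a maze key pickup that bots collect by overlapping its interaction sphere.
; The construction script reads a data table row to set the key's signature, name and color on a dynamic material instance.
; On BeginPlay it increments the game mode's KeysLeftInMaze count.
; On overlap with a BP_Bot it calls BotPickupKey on the bot, then decrements that count.
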(event `self.ReceiveBeginPlay`
  (bind _asbp_game_mode (cast `/Game/MazeGame/Blueprints/BP_GameMode` (`GameplayStatics.GetGameMode`)))
  (`/Engine/EditorBlueprintResources/StandardMacros.IsValid` _asbp_game_mode
    (:`Is Valid`
      (bind _result (`/Engine/EditorBlueprintResources/StandardMacros.IncrementInt` (`/Game/MazeGame/Blueprints/BP_GameMode.KeysLeftInMaze` _asbp_game_mode))
        (:`  `
          (set `/Game/MazeGame/Blueprints/BP_GameMode.KeysLeftInMaze` _result _asbp_game_mode))))))

(event `self.InteractionSphere.OnComponentBeginOverlap`
  (params (OverlappedComponent :type "PrimitiveComponent Object Reference") (OtherActor :type "Actor Object Reference") (OtherComp :type "PrimitiveComponent Object Reference") (OtherBodyIndex :type Integer) (bFromSweep :type Boolean) (SweepResult :type "HitResult Structure (by ref)"))
  (bind _asbp_bot (cast `/Game/MazeGame/Blueprints/AI/BP_Bot` OtherActor))
  (`/Engine/EditorBlueprintResources/StandardMacros.IsValid` _asbp_bot
    (:`Is Valid`
      (`MazeGameBot.BotPickupKey` _asbp_bot self)
      (bind _asbp_game_mode (cast `/Game/MazeGame/Blueprints/BP_GameMode` (`GameplayStatics.GetGameMode`)))
      (`/Engine/EditorBlueprintResources/StandardMacros.IsValid` _asbp_game_mode
        (:`Is Valid`
          (bind _result (`/Engine/EditorBlueprintResources/StandardMacros.DecrementInt` (`/Game/MazeGame/Blueprints/BP_GameMode.KeysLeftInMaze` _asbp_game_mode))
            (:`  `
              (set `/Game/MazeGame/Blueprints/BP_GameMode.KeysLeftInMaze` _result _asbp_game_mode))))))))

(fn `UserConstructionScript`
  (bind (_datatable _rowname) (break `DataTableRowHandle` (`self.KeyDataHandle`)))
  (bind _returnvalue (`KismetMaterialLibrary.CreateDynamicMaterialInstance` "/Game/MazeGame/Materials/M_BasicColor.M_BasicColor"))
  (bind _output_get (set `self.Material` _returnvalue))
  (`PrimitiveComponent.SetMaterial` (`self.Mesh`) 0 _output_get)
  (bind _returnvalue_2 (`|GetDataTableRow` _datatable _rowname)
    (:`then`
      (bind (_signature _color _name) (break `/Game/MazeGame/Data/FKeyDataRow` _returnvalue_2))
      (set `self.Signature` _signature)
      (`MaterialInstanceDynamic.SetVectorParameterValue` (`self.Material`) "Color" _color)
      (set `self.Name` _name))))